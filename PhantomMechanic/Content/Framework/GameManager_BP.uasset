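; Game instance manager that coordinates framework startup and hosts multiplayer sessions.
; Init marks the Game Instance ready, and components report through NotifyComponentReady, each setting a bit in a readiness bitmask.
; Once Game Instance, Game Mode, Game Data and Level are all ready, the state becomes Initalized and PhantomBaseMode_BP is notified.
; HostInstance creates a session with configurable connections and LAN setting, while JoinInstance and FindInstance are empty stubs.
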(event `self.ReceiveInit`
  (`KismetSystemLibrary.PrintString` "GameManger: Init called.")
  (`self.Notify Component Ready` "NewEnumerator0"))

(event `Notify Component Ready`
  (params (FComponent :type "/Game/Framework/_Enums/Framework_Components Enum" :default "NewEnumerator0"))
  (`self.Set Framework Component Ready` FComponent)
  (`self.Process Framework State`))

(event `Host Instance`
  ;[0 0 0 1 14] Handles the initalization for hosting an instance.
  (`KismetSystemLibrary.PrintString` "Host Instance: Called" true true (struct :`R` 1.0 :`B` 0.969686 :`A` 1.0))
  (`CreateSessionCallbackProxy.CreateSession` (`GameplayStatics.GetPlayerController` 0) (`self.Public Connections`) (`self.Lan?`)
    (:`OnSuccess`
      (`KismetSystemLibrary.PrintString` "Sucessfuly hosted instance." true true (struct :`R` 1.0 :`B` 0.969686 :`A` 1.0))
      (set `self.Session created?` true))
    (:`OnFailure`
      (`KismetSystemLibrary.PrintString` "Failed to host instance." true true (struct :`R` 1.0 :`B` 0.969686 :`A` 1.0)))))

(event `Join Instance`)

(event `Find Instance`)

(fn `Is Framework Ready?`
  (returns (Answer :type Boolean))
  (return (== (`self.Framework_InitalizaitonState`) (`|BitmaskLiteral` 15))))

(fn `Process Framework State`
  (locals (Changed :type Boolean))
  (`|ExecutionSequence`
    (:`then_0`
      (`KismetSystemLibrary.PrintString` "Processing framework state...")
      (switch `/Game/Framework/_Enums/FrameworkState` (`self.Current Framework State`)
        (:`NewEnumerator0`
          (bind _answer (`self.Is Framework Ready?`))
          (if _answer
            (set `self.Current Framework State` "NewEnumerator1")
            (`KismetSystemLibrary.PrintString` "Framework state set to initalized.")
            (set `local.Changed` true)))))
    (:`then_1`
      (if (`local.Changed`)
        (switch `/Game/Framework/_Enums/FrameworkState` (`self.Current Framework State`)
          (:`NewEnumerator1`
            (bind _asphantom_base_mode_bp (cast `/Game/Framework/PhantomBaseMode_BP` (`GameplayStatics.GetGameMode`)))
            (`/Game/Framework/PhantomBaseMode_BP.On Framework Initalized` _asphantom_base_mode_bp)))))))

(fn `Set Framework Component Ready`
  (params (Selection :type "/Game/Framework/_Enums/Framework_Components Enum" :default "NewEnumerator0"))
  (bind _framework_initalizaitonstate (`self.Framework_InitalizaitonState`))
  (`KismetSystemLibrary.PrintString` "Notify component ready called.")
  (`|ExecutionSequence`
    (:`then_0`
      (switch `/Game/Framework/_Enums/Framework_Components` Selection
        (:`NewEnumerator0`
          (set `self.Framework_InitalizaitonState` (`KismetMathLibrary.Or_IntInt` _framework_initalizaitonstate (`|BitmaskLiteral` 1))))
        (:`NewEnumerator1`
          (set `self.Framework_InitalizaitonState` (`KismetMathLibrary.Or_IntInt` _framework_initalizaitonstate (`|BitmaskLiteral` 2))))
        (:`NewEnumerator2`
          (set `self.Framework_InitalizaitonState` (`KismetMathLibrary.Or_IntInt` _framework_initalizaitonstate (`|BitmaskLiteral` 4))))
        (:`NewEnumerator3`
          (set `self.Framework_InitalizaitonState` (`KismetMathLibrary.Or_IntInt` _framework_initalizaitonstate (`|BitmaskLiteral` 8))))))))