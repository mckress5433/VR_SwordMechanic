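; ExoBody is a pawn Blueprint that assembles an exo body from separate hand and arm actors.
; On BeginPlay it spawns right and left ExoHand_BP actors at ExoOrigin, then an ExoArm_BP for each, passing it the matching hand.
; All four attach to ExoOrigin, and the left side reuses the same classes, mirrored by negative Z mesh scale.
; The possess event is an empty stub.
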(event `self.ReceiveBeginPlay`
  (bind _exo_hand_left (`self.Exo Hand Left`))
  (bind _exo_arm_left (`self.Exo Arm Left`))
  ;[1 1 1] Setup Arms and Hands
  (`|ExecutionSequence`
    (:`then_0`
      (`self.Spawn And Attach Hand` (`self.Exo Hand Right`))
      (`self.Spawn And Attach Hand` _exo_hand_left)
      (`SceneComponent.SetWorldScale3D` (`BodyPart.SkeletalMesh` _exo_hand_left) (1.0 1.0 -1.0)))
    (:`then_1`
      (`self.Spawn And Attach Arm` (`self.Exo Arm Right`) (`self.Exo Hand Right`))
      (`self.Spawn And Attach Arm` _exo_arm_left (`self.Exo Hand Left`))
      (`SceneComponent.SetWorldScale3D` (`BodyPart.SkeletalMesh` _exo_arm_left) (1.0 1.0 -1.0)))))

(event `ExoBody_Posses`
  (params (`Phantom Pawn` :type "/Game/Pawns/Phantom/PhantomPawn_BP Object Reference")))

(fn `Spawn And Attach Arm`
  (params (Arm :type "/Game/Pawns/ExoBody/Arms/ExoArm_BP Object Reference (by ref)") (Hand :type "/Game/Pawns/ExoBody/Hands/ExoHand_BP Object Reference"))
  (bind _returnvalue (`|SpawnActorFromClass` "/Game/Pawns/ExoBody/Arms/ExoArm_BP.ExoArm_BP_C" (`SceneComponent.K2_GetComponentToWorld` (`self.Exo_Origin`)) "Undefined" "OverrideRootScale" null self))
  (set `/Game/Pawns/ExoBody/Arms/ExoArm_BP.ExoHand` Hand _returnvalue)
  (`|VariableSetRef` Arm _returnvalue)
  (`self.K2_AttachToComponent` _returnvalue (`self.Exo_Origin`) "None" "SnapToTarget" "SnapToTarget" "SnapToTarget" true))

(fn `Spawn And Attach Hand`
  (params (InputPin :type "/Game/Pawns/ExoBody/Hands/ExoHand_BP Object Reference (by ref)"))
  (bind _returnvalue (`|SpawnActorFromClass` "/Game/Pawns/ExoBody/Hands/ExoHand_BP.ExoHand_BP_C" (`SceneComponent.K2_GetComponentToWorld` (`self.Exo_Origin`)) "Undefined" "OverrideRootScale" null self))
  (`|VariableSetRef` InputPin _returnvalue)
  (`self.K2_AttachToComponent` _returnvalue (`self.Exo_Origin`) "None" "KeepWorld" "KeepWorld" "KeepWorld" true))

(fn `UserConstructionScript`)