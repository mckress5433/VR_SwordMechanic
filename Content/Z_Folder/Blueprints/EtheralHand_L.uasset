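; Left ethereal hand actor that can split from its attached physical hand when overlapping blocking or parrying test objects.
; A block detaches the physical hand in place and reveals the ethereal mesh; a parry also offsets it against its velocity, capped by arm length.
; Overlapping that physical hand again snaps it back to the socket (marked WIP).
; The spawn-and-attach logic called from BeginPlay is unwired, so it never runs.
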(event `self.ReceiveBeginPlay`
  (`parent.ReceiveBeginPlay`)
  (`self.Create & Attach Physical Hand`))

(event `self.ReceiveTick`
  (params (DeltaSeconds :type "Float (single-precision)"))
  (`parent.ReceiveTick` DeltaSeconds))

(event `self.ReceiveActorBeginOverlap`
  (params (OtherActor :type "Actor Object Reference"))
  ;[1 1 1] Decouple check (works)
  (if (not (`self.Decoupled`))
    (cast `/Game/x-NewStuff/TestObjs/BlockingTestObj` OtherActor
      (:`then`
        (`self.BlockHand`))
      (:`CastFailed`
        (cast `/Game/x-NewStuff/TestObjs/ParryingTestObj` OtherActor)
        (`self.ParryHand`)))
    (else
      ;[1 1 1] Recouple check (wip)
      (bind _asphy_hand (cast `/Game/Z_Folder/Hand/Blueprints/PhyHand` OtherActor))
      (if (== _asphy_hand (`self.Physcial Hand`))
        (`self.Recouple` _asphy_hand)
        (set `self.Decoupled` false)))))

(fn `BlockHand`
  (`self.K2_DetachFromActor` (`self.Physcial Hand`) "KeepWorld" "KeepWorld" "KeepWorld")
  (`SceneComponent.SetVisibility` (`self.HandMesh`) true false)
  (set `self.Decoupled` true))

(fn `Create & Attach Physical Hand`)

(fn `ParryHand`
  (locals (Why :type "Vector Structure" :default (0.0 0.0 0.0)))
  (bind _physcial_hand (`self.Physcial Hand`))
  (bind _asphy_hand (cast `/Game/Z_Folder/Hand/Blueprints/PhyHand` _physcial_hand))
  (`self.K2_DetachFromActor` _physcial_hand "KeepWorld" "KeepWorld" "KeepWorld")
  (`SceneComponent.K2_SetWorldTransform` (`Actor.RootComponent` _physcial_hand) (`KismetMathLibrary.MakeTransform` (+ (`KismetMathLibrary.ClampVectorSize` (* (`/Game/Z_Folder/Hand/Blueprints/PhyHand.RealVelocity` _asphy_hand) -0.11) 0.0 (`self.ArmLength`)) (.location (`self.GetTransform` _physcial_hand))) (.rotation (`self.GetTransform` _physcial_hand)) (.scale (`self.GetTransform` _physcial_hand))) false false)
  (`SceneComponent.SetVisibility` (`self.HandMesh`) true false)
  (set `self.Decoupled` true))

(fn `Recouple`
  (params (`Physical Hand` :type "Actor Object Reference"))
  (bind _physcial_transformrule (`self.Physcial_TransformRule`))
  (`self.K2_SetActorTransform` `Physical Hand` (`SceneComponent.GetSocketTransform` (`self.HandMesh`) "PhysicalHandSocket" "RTS_World") false false)
  (`self.K2_AttachToComponent` `Physical Hand` (`self.HandMesh`) "PhysicalHandSocket" _physcial_transformrule _physcial_transformrule _physcial_transformrule true)
  (`SceneComponent.SetVisibility` (`self.HandMesh`) false false)
  (`SceneComponent.SetVisibility` (`Actor.RootComponent` (`self.Physcial Hand`)) true false))

(fn `UserConstructionScript`
  (`parent.UserConstructionScript`))