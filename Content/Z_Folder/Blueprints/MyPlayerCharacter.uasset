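; VR player character Blueprint that gives the player a pair of "Etheral" hand actors when play begins.
; BeginPlay calls SpawnAndAttachArms, which spawns the left and right hand classes at their motion controller transforms, always ignoring collision.
; Each hand then snaps to VROrigin rather than to its controller, keeping world scale.
; Only the right spawn sets the exposed Hand variable explicitly.
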(event `self.ReceiveBeginPlay`
  (`self.SpawnAndAttachArms`))

(fn `SpawnAndAttachArms`
  (`|ExecutionSequence`
    (:`then_0`
      (bind _returnvalue (`|SpawnActorFromClass` "/Game/Z_Folder/Blueprints/EtheralHand_L.EtheralHand_L_C" (`SceneComponent.K2_GetComponentToWorld` (`self.MotionController_L`)) "AlwaysSpawn" "OverrideRootScale" null "Left" null)) ; "Hand" is available by checking "Expose on Spawn in the variable on BP_MotionController.
      (`self.K2_AttachToComponent` _returnvalue (`self.VR_Origin`) "None" "SnapToTarget" "SnapToTarget" "KeepWorld" false))
    (:`then_1`
      (bind _returnvalue_2 (`|SpawnActorFromClass` "/Game/Z_Folder/Blueprints/EtheralHand_R.EtheralHand_R_C" (`SceneComponent.K2_GetComponentToWorld` (`self.MotionController_R`)) "AlwaysSpawn" "OverrideRootScale" null "Right" null)) ; "Hand" is available by checking "Expose on Spawn in the variable on BP_MotionController.
      (`self.K2_AttachToComponent` _returnvalue_2 (`self.VR_Origin`) "None" "SnapToTarget" "SnapToTarget" "KeepWorld" false))))

(fn `UserConstructionScript`)